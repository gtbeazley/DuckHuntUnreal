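; Player pawn that aims with its camera and destroys any Duck it points at, with no fire input required.
; Each Tick, a helper line-traces the Visibility channel along the camera's forward vector.
; DestinationMarker follows the hit location, or sits at the far end of the ray when nothing is hit.
; A hit actor that casts to Duck is destroyed immediately.
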(event `self.ReceiveTick`
  (params (DeltaSeconds :type "Float (single-precision)"))
  (bind _camera (`self.Camera`))
  (bind (_hitinfo _hitvalid) (`self.ComponentTraceForward` _camera))
  (if _hitvalid
    (bind (_bblockinghit _binitialoverlap _time _distance _location _impactpoint _normal _impactnormal _physmat _hitactor) (`GameplayStatics.BreakHitResult` _hitinfo))
    (`SceneComponent.K2_SetWorldLocation` (`self.DestinationMarker`) _location false false)
    (bind _asduck (cast `Duck` _hitactor))
    (`self.K2_DestroyActor` _asduck)
    (else
      (`SceneComponent.K2_SetWorldLocation` (`self.DestinationMarker`) (+ (`SceneComponent.K2_GetComponentLocation` _camera) (* (`SceneComponent.GetForwardVector` _camera) 10000.0)) false false))))

(fn `ComponentTraceForward`
  (params (ComponentToTrace :type "SceneComponent Object Reference"))
  (returns (HitInfo :type "HitResult Structure") (HitValid :type Boolean))
  (bind _returnvalue (`SceneComponent.K2_GetComponentLocation` ComponentToTrace))
  (bind (_outhit _returnvalue_2) (`KismetSystemLibrary.LineTraceSingle` _returnvalue (+ _returnvalue (* (`SceneComponent.GetForwardVector` ComponentToTrace) 10000.0)) "TraceTypeQuery1"))
  (return _outhit _returnvalue_2))

(fn `UserConstructionScript`)